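; BP_ZombieSpawner is a placed actor that spawns zombie AI with a configurable starting state.
; A looping timer set on BeginPlay drives spawning, which runs only while the spawner is active.
; Each zombie gets a tag built from the spawner's name and ID, used to count living spawns against a cap.
; Below the cap it spawns another just above itself; at the cap it waits or optionally destroys itself.
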(event Custom|Spawn%20AI
  (if (Variables|Default|GetActive)
    (bind _outactors (Actor|GetAllActorswithTag (Variables|Default|GetSpawnTag)))
    (if (>= (Utilities|Array|Length _outactors) (Variables|Default|GetSpawn%20Count))
      (if (Variables|Default|GetDestroy%20On%20End)
        (Actor|DestroyActor))
      (else
        (bind _returnvalue (Game|SpawnActorfromClass (Variables|Default|GetSpawn%20Class) (Math|Transform|MakeTransform (+ (Transformation|GetActorLocation) "0.000000,0.000000,60.000000") "0, 0, 0" "1.000000,1.000000,1.000000") "AlwaysSpawn" "MultiplyWithRoot" 0 (Variables|Default|GetStart%20Zombie%20State) 0))
        (Utilities|IsValid _returnvalue
          (:Is%20Valid
            (Utilities|Array|Add (Variables|/Script/Engine.Actor|GetTags _returnvalue) (Variables|Default|GetSpawnTag))))))))

(event EventBeginPlay
  (Variables|Default|SetSpawnTag (Utilities|String|StringToName (Utilities|String|Append (Utilities|GetObjectName self) (Variables|Default|GetSpawner%20ID))))
  (Utilities|Time|SetTimerbyEvent (EventDispatchers|CreateEvent :!event Custom|Spawn%20AI) (Variables|Default|GetDuration) true))

(fn ConstructionScript)