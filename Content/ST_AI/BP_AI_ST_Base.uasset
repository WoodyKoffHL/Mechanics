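; Base AI Blueprint that uses pawn sensing to pick a seen target and drive a StateTree.
; A macro sorts seen pawns into player, enemy (matched by TeamTag) or invalid.
; Player and enemy branches set the target and attack flag through DoOnce gates, then send a SeeTarget StateTree event.
; Invalid sightings clear both variables, and Tick prints the attack flag for debugging.
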(event OnSeePawn(PawnSensing)
  (params (Pawn :type Pawn%20Object%20Reference))
  (bind _pawn_seeing (Utilities|SeengMacro Pawn)
    (:Player
      (CallFunction|StartSeengPlayer _pawn_seeing)
      (Gameplay|StateTree|SendStateTreeEvent (Variables|Default|GetStateTree) (Utilities|Struct|MakeStateTreeEvent "(TagName=\"AI.StateTree.SeeTarget\")") :!class /Script/GameplayStateTreeModule.StateTreeComponent :!label _label))
    (:Enemie
      (CallFunction|StartSeengEnemie _pawn_seeing)
      (goto _label))
    (:Invalid
      (CallFunction|StopChasing))))

(event Custom|Start%20Seeng%20Enemie
  (params (Actor :type Actor%20Object%20Reference))
  (Utilities|FlowControl|DoOnce false
    (:Completed
      (Variables|Default|SetSeeing%20Target Actor)
      (Variables|Default|SetSeeing%20Target%20For%20Attack true))))

(event Custom|Start%20Seeng%20Player
  (params (Actor :type Actor%20Object%20Reference))
  (Utilities|FlowControl|DoOnce false
    (:Completed
      (Variables|Default|SetSeeing%20Target Actor)
      (Variables|Default|SetSeeing%20Target%20For%20Attack true))))

(event Custom|Stop%20Chasing
  (Variables|Default|SetSeeing%20Target 0)
  (Variables|Default|SetSeeing%20Target%20For%20Attack false))

(event EventBeginPlay)

(event Collision|EventActorBeginOverlap
  (params (OtherActor :type Actor%20Object%20Reference)))

(event EventTick
  (params (DeltaSeconds :type Float%20%28single-precision%29))
  (Development|PrintString (Utilities|String|ToString(Boolean) (Variables|Default|GetSeeing%20Target%20For%20Attack)) true true "(R=0.000000,G=0.660000,B=1.000000,A=1.000000)" 0.0))

(fn ConstructionScript)