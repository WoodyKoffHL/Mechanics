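; Climbing component that lets its owning character climb surfaces whose components are tagged "Climb", using mesh and character references passed in at init.
; A forward line trace from the Head socket detects climbable surfaces and broadcasts the result, also on an optional looping timer.
; Climbing toggles Flying movement, updates the AnimInstance through an interface and turns the character to the wall each tick.
; Losing the surface mid-climb plays a climb-up montage, then restores Walking.
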(event Custom|Init%20Component
  (params (Player%20Mesh%20Component :type Skeletal%20Mesh%20Component%20Object%20Reference) (Character :type Character%20Object%20Reference))
  ;[0.15 0.15 0.15 0.5] Инициализируем компонент через персонажа, добавляя его компоненты и ссылку
  (Variables|Default|SetPlayer%20Mesh%20Component Player%20Mesh%20Component)
  (Variables|Default|SetOwning%20Character Character))

(event Custom|Checking%20Climb%20Timer
  ;[0.15 0.15 0.15 0.5] Запускаем таймер для проверки, есть ли рядом объект, по которому можно карабкаться
  (CallFunction|CheckCanClimb))

(event Custom|Try%20Start%20Climb
  ;[0.15 0.15 0.15 0.5] Пытаемся начать лезть, в случае неудачи - Отменяем текущее состояние
  (if (not (Variables|Default|GetClimbing))
    (bind _can_climb (CallFunction|CheckCanClimb))
    (if _can_climb
      (Pawn|Components|CharacterMovement|SetMovementMode (Variables|/Script/Engine.Character|GetCharacterMovement (Variables|Default|GetOwning%20Character)) "MOVE_Flying" 0)
      (bind _output_get (Variables|Default|SetClimbing true))
      (Class|BPIClimbingSystem|SetClimbingonBPI(Message) (Components|SkeletalMesh|GetAnimInstance (Variables|Default|GetPlayer%20Mesh%20Component)) _output_get))
    (else
      (CallFunction|StopClimbing))))

(event Custom|Stop%20Climbing
  ;[0.15 0.15 0.15 0.5] Прекратить Карабканье
  (bind _output_get (Variables|Default|SetClimbing false))
  (Class|BPIClimbingSystem|SetClimbingonBPI(Message) (Components|SkeletalMesh|GetAnimInstance (Variables|Default|GetPlayer%20Mesh%20Component)) _output_get)
  (Pawn|Components|CharacterMovement|SetMovementMode (Variables|/Script/Engine.Character|GetCharacterMovement (Variables|Default|GetOwning%20Character)) "MOVE_Walking" 0))

(event Custom|Check%20In%20Climb
  (bind _owning_character (Variables|Default|GetOwning%20Character))
  (bind _returnvalue (Transformation|GetActorRotation _owning_character))
  ;[0.15 0.15 0.15 0.5 26] Проверяем каждый кадр - находимся ли мы перед объектом, по которому можно карабкаться
  (if (Variables|Default|GetClimbing)
    (bind (_can_climb _z_yaw) (CallFunction|CheckCanClimb))
    (if _can_climb
      (Transformation|SetActorRotation _owning_character (Math|Rotator|MakeRotator (.roll _returnvalue) (.pitch _returnvalue) _z_yaw))
      (else
        (Utilities|FlowControl|DoOnce false
          (:Completed
            (CallFunction|ClimbWallFront)))))))

(event Custom|Start%20Timer%20Focus%20Climb
  ;[0.15 0.15 0.15 0.5] Запускаем таймер для проверки, есть ли рядом объект, по которому можно карабкаться
  (Utilities|Time|SetTimerbyEvent (EventDispatchers|CreateEvent :!event Custom|Checking%20Climb%20Timer) 0.8 true))

(event Custom|Climb%20Wall%20Front
  (bind _owning_character (Variables|Default|GetOwning%20Character))
  (bind _returnvalue (Transformation|GetActorLocation _owning_character))
  (Utilities|FlowControl|Sequence
    (:then_0
      (CallFunction|GetForwardVector))
    (:then_1
      (Transformation|SetActorLocation _owning_character (Math|Vector|MakeVector (.x _returnvalue) (.y _returnvalue) (- (.z _returnvalue) 3e+01)) false false)
      (Animation|Montage|PlayMontage (Variables|Default|GetPlayer%20Mesh%20Component) "/Game/Demo/Mannequins/Anims/Climbing/AM_ClimbUP.AM_ClimbUP"
        (:then
          (Utilities|FlowControl|Delay 2.0)
          (CallFunction|StopClimbing)
          (CallFunction|ResetClimbWallFront))))))

(event Custom|Reset%20Climb%20Wall%20Front
  ;[0.15 0.15 0.15 0.5 26] Проверяем каждый кадр - находимся ли мы перед объектом, по которому можно карабкаться
  (Utilities|FlowControl|DoOnce false) ; enters at Reset
)

(event EventBeginPlay)

(event EventTick
  (params (DeltaSeconds :type Float%20%28single-precision%29))
  (CallFunction|CheckinClimb))

(fn CheckCanClimb
  (bind _player_mesh_component (Variables|Default|GetPlayer%20Mesh%20Component))
  (bind _returnvalue (Transformation|GetSocketLocation _player_mesh_component "Head"))
  (Utilities|IsValid _player_mesh_component
    (:Is%20Valid
      (bind (_outhit _returnvalue_2) (Collision|LineTraceByChannel _returnvalue (+ _returnvalue (* (Math|Vector|GetForwardVector (Variables|/Script/Engine.Actor|GetRootComponent (Variables|Default|GetOwning%20Character))) 5e+01)) "TraceTypeQuery1" false 0 "None"))
      (if _returnvalue_2
        (Default|CallOnCheckCanClimb (Components|ComponentHasTag (.HitComponent (Collision|BreakHitResult _outhit)) "Climb"))
        (bind _output_get (Variables|Default|SetNormal (.Normal (Collision|BreakHitResult _outhit))))
        (return (Components|ComponentHasTag (.HitComponent (Collision|BreakHitResult _outhit)) "Climb") (+ (.yaw (Math|Rotator|MakeRotfromX _output_get)) 1.8e+02))
        (else
          (Default|CallOnCheckCanClimb false)
          (return false 0.0))))
    (:Is%20Not%20Valid
      (Default|CallOnCheckCanClimb false)
      (return false 0.0))))

(fn GetForwardVector)