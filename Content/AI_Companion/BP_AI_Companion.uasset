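; AI companion actor that follows a Character and, when called, marks active targets in the level.
; Each Tick it snaps to the Character and spins its compass and spring arm, while a DoOnce-gated Timeline moves the compass up or down.
; CallCompanionBPI destroys previous markers, spawns BP_Target at every actor tagged both Target and Active, then starts a short timer.
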(event Custom|End%20Checking%20Targets
  (for _array_element (Variables|Default|GetTargets)
    (Utilities|IsValid _array_element
      (:Is%20Valid
        (Actor|DestroyActor _array_element)))))

(event EventBeginPlay)

(event Collision|EventActorBeginOverlap
  (params (OtherActor :type Actor%20Object%20Reference)))

(event EventTick
  (params (DeltaSeconds :type Float%20%28single-precision%29))
  (Transformation|AddLocalRotation (Variables|Default|GetCompas) "0.000000,3.000000,0.000000" false false)
  (Transformation|AddLocalRotation (Variables|Default|GetSpringArm) "0.000000,1.000000,0.000000" false false)
  (bind _character (Variables|Default|GetCharacter)
    (:then
      (Transformation|SetActorLocation (Transformation|GetActorLocation _character) false false)
      (Utilities|FlowControl|DoOnce false :!label _label
        (:Completed
          (if (< (.z (Variables|/Script/Engine.SceneComponent|GetRelativeLocation (Variables|Default|GetCompas))) 2.0)
            (bind _newtrack_0 (Timeline|Timeline Play)
              (:Update
                (Transformation|SetRelativeLocation (Variables|Default|GetCompas) (Math|Vector|MakeVector 0.0 0.0 _newtrack_0) false false))
              (:Finished
                (goto _label Reset)))
            (else
              (Timeline|Timeline Reverse))))))
    (:else)))

(event EventCallCompanionBPI
  (params (Caller :type Actor%20Object%20Reference))
  (CallFunction|EndCheckingTargets)
  (bind _outactors (Actor|GetAllActorswithTag "Target"))
  (for _array_element _outactors
    (if (Actor|ActorHasTag _array_element "Active")
      (bind _returnvalue (Game|SpawnActorfromClass "/Game/AI_Companion/BP_Target.BP_Target_C" (Math|Transform|MakeTransform (Transformation|GetActorLocation _array_element) "0, 0, 0" "1.000000,1.000000,1.000000") "AlwaysSpawn" "MultiplyWithRoot" 0 0))
      (Utilities|Array|Add (Variables|Default|GetTargets) _returnvalue)))
  (Utilities|Time|SetTimerbyEvent (EventDispatchers|CreateEvent :!event Custom|End%20Checking%20Targets) 5.0))

(fn ConstructionScript)