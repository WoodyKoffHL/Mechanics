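; BP_Small is a small destroyable wall that breaks into physics debris when its explode-destroy event fires.
; BeginPlay gathers nine pre-placed cube components into an array as the fragments.
; The event hides the intact Wall and disables its collision, then reveals the cubes, enables their physics and impulses them opposite the supplied direction.
; A timer destroys the whole actor a few seconds later.
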(event Custom|Destroy%20Components
  (Actor|DestroyActor))

(event EventBeginPlay
  (|CallParentFunction)
  (Variables|Default|SetCubes (Utilities|Array|MakeArray (Variables|Default|GetCube_005) (Variables|Default|GetCube_008) (Variables|Default|GetCube_007) (Variables|Default|GetCube_006) (Variables|Default|GetCube_009) (Variables|Default|GetCube_004) (Variables|Default|GetCube_003) (Variables|Default|GetCube_002) (Variables|Default|GetCube_001))))

(event Collision|EventActorBeginOverlap
  (params (OtherActor :type Actor%20Object%20Reference))
  (|CallParentFunction OtherActor) ; This node is disabled and will not be called.\nDrag off pins to build functionality.
)

(event EventTick
  (params (DeltaSeconds :type Float%20%28single-precision%29))
  (|CallParentFunction DeltaSeconds) ; This node is disabled and will not be called.\nDrag off pins to build functionality.
)

(event EventCAExploydeDestroy
  (params (Dir :type Vector :default "0, 0, 0"))
  (bind _wall (Variables|Default|GetWall))
  (Collision|SetCollisionEnabled _wall "NoCollision")
  (Rendering|SetVisibility _wall false false)
  (for _array_element (Variables|Default|GetCubes)
    (Rendering|SetVisibility _array_element true false)
    (Collision|SetCollisionObjectType _array_element "ECC_WorldDynamic")
    (Physics|SetSimulatePhysics _array_element true)
    (Physics|AddImpulse _array_element (* Dir -4e+02) "None" false))
  (Utilities|Time|SetTimerbyEvent (delegate Custom|Destroy%20Components) 3.0))

(fn ConstructionScript
  (|CallParentFunction))