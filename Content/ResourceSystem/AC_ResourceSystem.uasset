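; AC_ResourceSystem is a resource-tracking component that keeps a main resource total and a separate collectible count.
; Add events increase each total, and dispatchers broadcast the new main total or whether the collectible count has reached its required threshold.
; The collected dispatcher fires on every collect addition, passing that threshold flag.
; Tick prints the main resource every frame as debug output.
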(event Custom|Add%20Main%20Resource
  (params (Amount :type Integer))
  (bind _output_get (Variables|Default|SetMainResource (+ (Variables|Default|GetMainResource) Amount)))
  (Default|CallResourceAdded _output_get))

(event Custom|Add%20Collect%20Resource
  (params (Amount :type Integer))
  (bind _output_get (Variables|Default|SetCoolect%20Resource (+ (Variables|Default|GetCoolect%20Resource) Amount)))
  (bind _output_get_2 (Variables|Default|SetHave%20Collect (>= _output_get (Variables|Default|GetNeed%20for%20Collect))))
  (Default|CallCollectedObject _output_get_2))

(event EventBeginPlay)

(event EventTick
  (params (DeltaSeconds :type Float%20%28single-precision%29))
  (Development|PrintString (Utilities|String|ToString(Integer) (Variables|Default|GetMainResource)) true true "(R=0.000000,G=0.660000,B=1.000000,A=1.000000)" 0.0))