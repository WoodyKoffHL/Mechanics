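; Base actor for placeable RTS buildings, acting as a placement preview until built.
; While unbuilt, Tick traces from the cursor or screen center and snaps the actor to the grid.
; Base types box-trace for overlaps, while Resource types require a tagged actor and copy its transform, tinting the cube green or red.
; Interface calls rotate it in 45-degree yaw steps and confirm placement, enabling collision and turning it white.
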(event EventBeginPlay
  (Collision|SetCollisionEnabled (Variables|Default|GetCube) (select (Variables|Gameplay|GetBuilded) "QueryAndPhysics" "NoCollision")))

(event Collision|EventActorBeginOverlap
  (params (OtherActor :type Actor%20Object%20Reference)))

(event EventTick
  (params (DeltaSeconds :type Float%20%28single-precision%29))
  (if (not (Variables|Gameplay|GetBuilded))
    (switch Utilities|FlowControl|Switch|SwitchonEN_BuildType (Variables|BuildType|GetBuild%20Type)
      (:NewEnumerator0
        (BUILDING|TraceandPlacePerBUILD))
      (:NewEnumerator1
        (BUILDING|TraceResourcePerBUILD)))))

(event EventBPIRotateBuild
  (bind _returnvalue (Transformation|GetActorRotation))
  (Transformation|SetActorRotation (Math|Rotator|MakeRotator (.roll _returnvalue) (.pitch _returnvalue) (+ (.yaw _returnvalue) 45.0))))

(fn ConstructionScript)

(fn LineTraceStart-End
  (bind _returnvalue (Game|GetPlayerController 0))
  (bind _returnvalue_2 (Viewport|GetViewportSize))
  (bind _returnvalue_3 (/ (.y _returnvalue_2) 2.0))
  (bind _returnvalue_4 (/ (.x _returnvalue_2) 2.0))
  (bind _worldposition (Class|GameplayStatics|DeprojectScreentoWorld _returnvalue (Math|Vector2D|MakeVector2D _returnvalue_4 _returnvalue_3)))
  (return _worldposition (+ _worldposition (* (Math|Vector|GetForwardVector (Camera|GetCameraRotation (Game|GetPlayerCameraManager 0))) 9e+03))))

(fn GetHitResultbyInput
  (bind (_start _end) (Technical|LineTraceStart-End))
  (if (Variables|/Script/Engine.PlayerController|GetbShowMouseCursor (Variables|Components|GetPlayer%20Controller))
    (return (.HitResult (Game|Player|GetHitResultUnderCursorbyChannel (Variables|Components|GetPlayer%20Controller) "TraceTypeQuery2" true)))
    (else
      (bind _outhit (Collision|LineTraceByChannel _start _end "TraceTypeQuery1" false 0 "None"))
      (return _outhit))))

(fn TraceandPlacePerBUILD
  (if (not (Variables|Gameplay|GetBuilded))
    (Variables|Components|GetPlayer%20Controller
      (:then
        (bind _hitresult (Technical|GetHitResultbyInput))
        (if (.bBlockingHit (Collision|BreakHitResult _hitresult))
          (Transformation|SetActorLocation (Default|GetGridLocation (Variables|Default|GetBPC_Grid) (Math|Vector|MakeVector (.X (Math|Vector|BreakVector (.Location (Collision|BreakHitResult _hitresult)))) (.Y (Math|Vector|BreakVector (.Location (Collision|BreakHitResult _hitresult)))) (.Z (Math|Vector|BreakVector (.Location (Collision|BreakHitResult _hitresult)))))) false false)
          (bind _returnvalue (Collision|BoxTraceByChannel (+ (Default|GetGridLocation (Variables|Default|GetBPC_Grid) (Math|Vector|MakeVector (.X (Math|Vector|BreakVector (.Location (Collision|BreakHitResult _hitresult)))) (.Y (Math|Vector|BreakVector (.Location (Collision|BreakHitResult _hitresult)))) (.Z (Math|Vector|BreakVector (.Location (Collision|BreakHitResult _hitresult)))))) "0.000000,0.000000,950.000000") (+ (Default|GetGridLocation (Variables|Default|GetBPC_Grid) (Math|Vector|MakeVector (.X (Math|Vector|BreakVector (.Location (Collision|BreakHitResult _hitresult)))) (.Y (Math|Vector|BreakVector (.Location (Collision|BreakHitResult _hitresult)))) (.Z (Math|Vector|BreakVector (.Location (Collision|BreakHitResult _hitresult)))))) "0.000000,0.000000,950.000000") "600.000000,600.000000,900.000000" (Transformation|GetActorRotation) "TraceTypeQuery1" true 0 "ForDuration"))
          (bind _output_get (Variables|Gameplay|SetCan%20Build (not _returnvalue)))
          (Rendering|Material|SetMaterial (Variables|Default|GetCube) 0 (select _output_get "/Game/RTS_Template/Materials/MI_OpacityGreen.MI_OpacityGreen" "/Game/RTS_Template/Materials/MI_OpacityRed.MI_OpacityRed"))))
      (:else))))

(fn TraceResourcePerBUILD
  (if (not (Variables|Gameplay|GetBuilded))
    (Variables|Components|GetPlayer%20Controller
      (:then
        (bind _hitresult (Technical|GetHitResultbyInput))
        (if (.bBlockingHit (Collision|BreakHitResult _hitresult))
          (Transformation|SetActorLocation (Default|GetGridLocation (Variables|Default|GetBPC_Grid) (Math|Vector|MakeVector (.X (Math|Vector|BreakVector (.Location (Collision|BreakHitResult _hitresult)))) (.Y (Math|Vector|BreakVector (.Location (Collision|BreakHitResult _hitresult)))) (.Z (Math|Vector|BreakVector (.Location (Collision|BreakHitResult _hitresult)))))) false false)
          (bind _output_get (Variables|Gameplay|SetCan%20Build (Actor|ActorHasTag (.HitActor (Collision|BreakHitResult _hitresult)) (Variables|BuildType|GetResource%20Tag))))
          (if _output_get
            (Transformation|SetActorTransform (Transformation|GetActorTransform (.HitActor (Collision|BreakHitResult _hitresult))))
            (Rendering|Material|SetMaterial (Variables|Default|GetCube) 0 "/Game/RTS_Template/Materials/MI_OpacityGreen.MI_OpacityGreen")
            (Variables|Gameplay|SetCan%20Build true)
            (else
              (Rendering|Material|SetMaterial (Variables|Default|GetCube) 0 "/Game/RTS_Template/Materials/MI_OpacityRed.MI_OpacityRed")
              (Variables|Gameplay|SetCan%20Build false)))))
      (:else))))

(fn BPIBuildStart
  (bind _can_build (Variables|Gameplay|GetCan%20Build))
  (if _can_build
    (bind _output_get (Variables|Gameplay|SetBuilded _can_build))
    (Rendering|Material|SetMaterial (Variables|Default|GetCube) 0 "/Game/RTS_Template/Materials/MI_OpacityWhite.MI_OpacityWhite")
    (Collision|SetCollisionEnabled (Variables|Default|GetCube) "QueryAndPhysics")
    (return _output_get)
    (else
      (return false))))