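; RTS camera pawn that pans and zooms over the map with a visible mouse cursor, using the IMC_RTS Enhanced Input context added on BeginPlay.
; Move input drives FloatingPawnMovement, with a fast-move action raising max speed while held, and zoom steps the SpringArm length within limits.
; Mouse axis events run a movementMouseXY macro that detects the cursor in the outer tenth of the viewport; only MouseX applies the resulting local offset.
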(event Input|EnhancedActionEvents|EnhancedInputActionIA_RTS_CameraMoving
  (params (ActionValue :type Vector%202D%20Structure) (ElapsedSeconds :type Float%20%28double-precision%29) (TriggeredSeconds :type Float%20%28double-precision%29) (InputAction :type Input%20Action%20Object%20Reference :default "/Game/RTS_Template/Input/IA_RTS_CameraMoving.IA_RTS_CameraMoving"))
  (bind (_x _y) (Math|Vector2D|BreakVector2D ActionValue))
  ;[0.15 0.15 0.15 0.5] Camera Manual Move
  (:Triggered
    (Pawn|Input|AddMovementInput (Transformation|GetActorForwardVector) _y false)
    (Pawn|Input|AddMovementInput (Transformation|GetActorRightVector) _x false)))

(event Input|EnhancedActionEvents|EnhancedInputActionIA_RTS_FastMoving
  (params (ActionValue :type Boolean) (ElapsedSeconds :type Float%20%28double-precision%29) (TriggeredSeconds :type Float%20%28double-precision%29) (InputAction :type Input%20Action%20Object%20Reference :default "/Game/RTS_Template/Input/IA_RTS_FastMoving.IA_RTS_FastMoving"))
  (bind _floatingpawnmovement (Variables|Default|GetFloatingPawnMovement))
  ;[0.15 0.15 0.15 0.5] Camera Manual Move
  (:Started
    (Variables|/Script/Engine.FloatingPawnMovement|SetMaxSpeed _floatingpawnmovement 6e+03))
  (:Completed
    (Variables|/Script/Engine.FloatingPawnMovement|SetMaxSpeed _floatingpawnmovement 3e+03)))

(event Input|EnhancedActionEvents|EnhancedInputActionIA_RTS_Zoom
  (params (ActionValue :type Float%20%28double-precision%29) (ElapsedSeconds :type Float%20%28double-precision%29) (TriggeredSeconds :type Float%20%28double-precision%29) (InputAction :type Input%20Action%20Object%20Reference :default "/Game/RTS_Template/Input/IA_RTS_Zoom.IA_RTS_Zoom"))
  (bind _springarm (Variables|Default|GetSpringArm))
  ;[0.15 0.15 0.15 0.5] Zoom
  (:Triggered
    (Variables|/Script/Engine.SpringArmComponent|SetTargetArmLength _springarm (Math|Float|Clamp(Float) (+ (Variables|/Script/Engine.SpringArmComponent|GetTargetArmLength _springarm) (select (> ActionValue 0.6) -1e+02 1e+02)) 2e+02 2.5e+03))))

(event EventBeginPlay
  (bind _returnvalue (Game|GetPlayerController 0))
  (Utilities|IsValid _returnvalue
    (:Is%20Valid
      (Input|AddMappingContext (PlayerController|LocalPlayerSubsystems|GetEnhancedInputLocalPlayerSubsystem _returnvalue) "/Game/RTS_Template/Input/IMC_RTS.IMC_RTS" 0 "(bIgnoreAllPressedKeysUntilRelease=True,bForceImmediately=False,bNotifyUserSettings=False)")
      (Variables|/Script/Engine.PlayerController|SetbShowMouseCursor (Game|GetPlayerController 0) true))))

(event Collision|EventActorBeginOverlap
  (params (OtherActor :type Actor%20Object%20Reference)))

(event EventTick
  (params (DeltaSeconds :type Float%20%28single-precision%29)))

(event Input|MouseEvents|MouseX
  (params (AxisValue :type Float%20%28single-precision%29))
  ;[0.15 0.15 0.15 0.5] Camera Manual Move
  (bind (_speed_x _speed_y) (Utilities|MovementMouseXY)
    (:Return
      (Transformation|AddActorLocalOffset (Math|Vector|MakeVector (* _speed_x 2.0) (* _speed_y 2.0) 0.0) false false))))

(event Input|MouseEvents|MouseY
  (params (AxisValue :type Float%20%28single-precision%29))
  ;[0.15 0.15 0.15 0.5] Camera Manual Move
  (Utilities|MovementMouseXY) ; enters at Move Y
)

(fn ConstructionScript)