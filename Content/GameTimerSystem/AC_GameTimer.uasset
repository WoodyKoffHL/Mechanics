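; Game timer component that runs a countdown of the current level time and announces its progress through event dispatchers.
; StartTimerWithTime sets the time, then StartTimer creates a looping one-second timer and broadcasts TimerStarted.
; TimerImplement decrements the time and broadcasts TimeImplement as the per-tick update.
; At zero or below it broadcasts TimeOut and calls StopTimer, which clears and invalidates the timer handle.
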(event Custom|Timer%20Implement
  ;[0.15 0.15 0.15 0.5] Implement Timer
  (Math|Float|DecrementFloat (Variables|Default|GetCurrent%20Level%20Time)
    (:%20%20
      (Default|CallTimeImplement)
      (if (<= (Variables|Default|GetCurrent%20Level%20Time) 0.0)
        (Default|CallTimeOut)
        (CallFunction|StopTimer)))))

(event Custom|Stop%20Timer
  ;[0.15 0.15 0.15 0.5] Stop Timer
  (Utilities|Time|ClearandInvalidateTimerbyHandle (Variables|Default|GetTimer%20Handle)))

(event Custom|Start%20Timer
  ;[0.15 0.15 0.15 0.5] Start Timer
  (bind _returnvalue (Utilities|Time|SetTimerbyEvent (EventDispatchers|CreateEvent :!event Custom|Timer%20Implement) 1.0 true))
  (Variables|Default|SetTimer%20Handle _returnvalue)
  (Default|CallTimerStarted))

(event Custom|Start%20Timer%20With%20Time
  (params (Time :type Float%20%28double-precision%29))
  ;[0.15 0.15 0.15 0.5] Start Timer
  (Variables|Default|SetCurrent%20Level%20Time Time)
  (CallFunction|StartTimer))