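; Documentation Blueprint showing how an owner Actor, ideally the Game Mode, uses the game timer system through its interface, with Russian usage notes.
; StartGameTimerBPI adds the AC_GameTimer component, while the other start, stop and fail events and both getters are empty stubs.
; Unconnected example nodes show binding to timer started, time change and time-out delegates, and fetching the component or current time from the Game Mode via interface messages.
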(event EventStartGameTimerBPI
  ;[0 0 0 0.5] For Actor Owner - Для Владельца компонента
  ;;[0.15 0.15 0.15 0.5] Добавить Компонент через интерфейс. После добавления, таймер начинает работу в Actor. Рекомендую использовать в Game Mode для времени - связанного с игрой. Для других применений - лучше создать дочерний класс компонента
  (AddComponent|AddACGameTimer))

(event EventStopTimerBPI
  ;[0 0 0 0.5] For Actor Owner - Для Владельца компонента
  ;;[0.15 0.15 0.15 0.5] Использование функции можно Изтолковать по разному. Остановить таймер, например, если уровень пройден.
)

(event EventFailandStopTimerBPI
  ;[0 0 0 0.5] For Actor Owner - Для Владельца компонента
  ;;[0.15 0.15 0.15 0.5] Использование функции - Остановить таймер, например, если Игра проиграна.
)

(event EventStartGameTimerwithTimeBPI
  (params (Time :type Float%20%28double-precision%29))
  ;[0 0 0 0.5] For Actor Owner - Для Владельца компонента
  ;;[0.15 0.15 0.15 0.5] Старт Таймера с определенным временем
)

(fn ConstructionScript)

(fn GetCurrentTimeBPI
  (return 0.0))

(fn GetGameTimerComponentBPI
  (return 0))