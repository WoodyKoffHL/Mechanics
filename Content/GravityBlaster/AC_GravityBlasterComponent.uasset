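; Gravity gun component that lets its owner pull, hold and launch physics objects from the camera view.
; On BeginPlay it sets up the blaster mesh and physics handle, removing itself if no camera exists.
; Pull toggles grabbing of sphere-traced BPI_Grabbable objects, which Tick holds before the camera.
; Push launches the held object forward, or impulses a traced physics object toward the camera, notifying objects through interface messages.
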(event EventBeginPlay
  (bind _returnvalue (Components|GetOwner))
  (bind _returnvalue_2 (Actor|GetComponentbyClass _returnvalue "/Script/Engine.CameraComponent"))
  (Class|BPIGravityBlaster|SetGravityBlasterBPI(Message) (Components|GetOwner) (Variables|Default|GetBlaster%20Mesh) (Variables|Default|GetSocket%20Name))
  (bind _returnvalue_3 (Game|AddComponentbyClass (Components|GetOwner) "/Script/Engine.PhysicsHandleComponent"))
  (bind _output_get (Variables|Default|SetPhysics%20Handle _returnvalue_3))
  (Class|PhysicsHandleComponent|SetInterpolationSpeed _output_get (Variables|Default|GetInterpolation%20Speed))
  (Utilities|IsValid _returnvalue_2
    (:Is%20Valid
      (Variables|Default|SetCamera%20Component _returnvalue_2))
    (:Is%20Not%20Valid
      (Components|DestroyComponent))))

(event EventTick
  (params (DeltaSeconds :type Float%20%28single-precision%29))
  (bind _camera_component (Variables|Default|GetCamera%20Component))
  (bind _hold_object_distance (Variables|Default|GetHold%20Object%20Distance))
  (bind _camera_component_2 (Variables|Default|GetCamera%20Component))
  (bind _returnvalue (Math|Vector|GetForwardVector _camera_component))
  (bind _returnvalue_2 (Transformation|GetWorldLocation _camera_component_2))
  (bind _returnvalue_3 (* _returnvalue _hold_object_distance))
  (bind _returnvalue_4 (+ _returnvalue_2 _returnvalue_3))
  (Variables|Default|GetGrabbed%20Component
    (:then
      (Class|PhysicsHandleComponent|SetTargetLocationandRotation (Variables|Default|GetPhysics%20Handle) _returnvalue_4 (Math|Rotator|FindLookatRotation _returnvalue_2 _returnvalue_4)))
    (:else)))

(fn ReleaseGrabbedObject
  (Physics|Components|PhysicsHandle|ReleaseComponent (Variables|Default|GetPhysics%20Handle))
  (bind _grabbed_component (Variables|Default|GetGrabbed%20Component)
    (:then
      (Class|BPIGrabbable|OnReleaseObjectBPI(Message) (Components|GetOwner _grabbed_component))
      (Variables|Default|SetGrabbed%20Component 0))
    (:else
      _))
  (Default|CallReleasedObject))

(fn PullObject
  (bind _camera_component (Variables|Default|GetCamera%20Component))
  (bind _physics_handle (Variables|Default|GetPhysics%20Handle))
  (bind _returnvalue (Transformation|GetWorldLocation _camera_component))
  (Variables|Default|GetGrabbed%20Component
    (:then
      (CallFunction|ReleaseGrabbedObject))
    (:else
      (bind (_outhit _returnvalue_2) (Collision|SphereTraceByChannel _returnvalue (+ _returnvalue (* (Math|Vector|GetForwardVector _camera_component) (Variables|Default|GetMax%20Pull%20Distance))) 15.0 "TraceTypeQuery1" true (Utilities|Array|MakeArray (Components|GetOwner)) "ForDuration"))
      (if _returnvalue_2
        (if (Utilities|DoesObjectImplementInterface (.HitActor (Collision|BreakHitResult _outhit)) "/Game/GravityBlaster/Interfaces/BPI_Grabbable.BPI_Grabbable_C")
          (Physics|Components|PhysicsHandle|GrabComponentatLocationwithRotation _physics_handle (.HitComponent (Collision|BreakHitResult _outhit)) "None" (Transformation|GetWorldLocation (.HitComponent (Collision|BreakHitResult _outhit))) (Transformation|GetWorldRotation (.HitComponent (Collision|BreakHitResult _outhit))))
          (Variables|Default|SetGrabbed%20Component (Class|PhysicsHandleComponent|GetGrabbedComponent _physics_handle))
          (Class|BPIGrabbable|OnPullObjectBPI(Message) (.HitActor (Collision|BreakHitResult _outhit)))
          (Default|CallPulledObject))))))

(fn PushObject
  (bind _camera_component (Variables|Default|GetCamera%20Component))
  (bind _returnvalue (Transformation|GetWorldLocation _camera_component))
  (bind _grabbed_component (Variables|Default|GetGrabbed%20Component)
    (:then
      (Physics|AddImpulse _grabbed_component (* (Math|Vector|GetForwardVector (Variables|Default|GetCamera%20Component)) (Variables|Default|GetPush%20Strength)) "None" true)
      (Class|BPIGrabbable|OnPushObjectBPI(Message) (Components|GetOwner (Variables|Default|GetGrabbed%20Component)))
      (CallFunction|ReleaseGrabbedObject))
    (:else
      (bind (_outhit _returnvalue_2) (Collision|SphereTraceByChannel _returnvalue (+ _returnvalue (* (Math|Vector|GetForwardVector _camera_component) (Variables|Default|GetMax%20Pull%20Distance))) 15.0 "TraceTypeQuery1" false 0 "None"))
      (if _returnvalue_2
        (Class|BPIGrabbable|OnPushObjectBPI(Message) (.HitActor (Collision|BreakHitResult _outhit)))
        (if (Physics|IsSimulatingPhysics (.HitComponent (Collision|BreakHitResult _outhit)) "None")
          (Physics|AddImpulse (.HitComponent (Collision|BreakHitResult _outhit)) (* (Math|Vector|GetUnitDirection(Vector) (.ImpactPoint (Collision|BreakHitResult _outhit)) (.TraceStart (Collision|BreakHitResult _outhit))) (Variables|Default|GetMax%20Pull%20Distance)) "None" true))))))