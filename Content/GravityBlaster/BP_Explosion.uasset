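; BP_Explosion is a one-shot explosion actor that detonates on BeginPlay, playing a particle and sound effect.
; A sphere trace applies heavy point damage to hit dynamic objects, physics bodies and pawns, and sends grabbables a delayed-destroy interface message.
; A radial force component, added at runtime, fires a velocity-change impulse over the same radius, excluding pawns, and the actor destroys itself next tick.
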(event Custom|Explode%20Effects
  (Effects|SpawnEmitteratLocation "/Engine/Tutorial/SubEditors/TutorialAssets/TutorialParticleSystem.TutorialParticleSystem" (Transformation|GetActorLocation))
  (Audio|PlaySoundatLocation "/Engine/EditorSounds/GamePreview/EjectFromPlayer.EjectFromPlayer" (Transformation|GetActorLocation) "0, 0, 0" 1.0 1.0 0.0 0 0 0 0))

(event EventBeginPlay
  (bind _returnvalue (Transformation|GetActorLocation))
  (CallFunction|ExplodeEffects)
  (bind _outhits (Collision|MultiSphereTraceForObjects _returnvalue _returnvalue (Variables|Default|GetRadius) (Utilities|Array|MakeArray "ObjectTypeQuery2" "ObjectTypeQuery4" "ObjectTypeQuery3") false 0 "None"))
  (for _array_element _outhits
    (Game|Damage|ApplyPointDamage (.HitActor (Collision|BreakHitResult _array_element)) 5e+02 (.ImpactPoint (Collision|BreakHitResult _array_element)) _array_element 0 0 "/Game/GravityBlaster/Damage/DT_ExploydDamage.DT_ExploydDamage_C")
    (if (Utilities|DoesObjectImplementInterface (.HitActor (Collision|BreakHitResult _array_element)) "/Game/GravityBlaster/Interfaces/BPI_Grabbable.BPI_Grabbable_C")
      (Class|BPIGrabbable|DelayedDestroyBPI(Message) (.HitActor (Collision|BreakHitResult _array_element)))))
  (bind _returnvalue_2 (AddComponent|AddRadialForceComponent false))
  (Variables|/Script/Engine.RadialForceComponent|SetRadius _returnvalue_2 (Variables|Default|GetRadius))
  (Variables|/Script/Engine.RadialForceComponent|SetImpulseStrength _returnvalue_2 (Variables|Default|GetImpulse%20Strength))
  (Variables|/Script/Engine.RadialForceComponent|SetbImpulseVelChange _returnvalue_2 true)
  (Class|RadialForceComponent|RemoveObjectTypetoAffect _returnvalue_2 "ObjectTypeQuery3")
  (Class|RadialForceComponent|FireImpulse _returnvalue_2)
  (Utilities|FlowControl|DelayUntilNextTick)
  (Actor|DestroyActor))

(fn ConstructionScript)