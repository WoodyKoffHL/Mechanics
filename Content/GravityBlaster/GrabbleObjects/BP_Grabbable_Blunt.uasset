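; BP_Grabbable_Blunt is a grabbable object variant for the gravity blaster that deals blunt damage when it hits something.
; It extends its parent's hit-object interface event, then applies fixed point damage to the hit actor.
; The damage direction is the inverted hit normal scaled by the inherited impulse strength.
; Its other events and construction script add nothing beyond the parent.
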(event EventBeginPlay
  (|CallParentFunction) ; This node is disabled and will not be called.\nDrag off pins to build functionality.
)

(event Collision|EventActorBeginOverlap
  (params (OtherActor :type Actor%20Object%20Reference))
  (|CallParentFunction OtherActor) ; This node is disabled and will not be called.\nDrag off pins to build functionality.
)

(event EventTick
  (params (DeltaSeconds :type Float%20%28single-precision%29))
  (|CallParentFunction DeltaSeconds) ; This node is disabled and will not be called.\nDrag off pins to build functionality.
)

(event EventOnHitObjectBPI
  (params (Hit%20Result :type Hit%20Result%20Structure))
  (bind (_bblockinghit _binitialoverlap _time _distance _location _impactpoint _normal _impactnormal _physmat _hitactor) (Collision|BreakHitResult Hit%20Result))
  (|CallParentFunction Hit%20Result)
  (Game|Damage|ApplyPointDamage _hitactor 6e+01 (* _normal (Variables|Default|GetImpulse%20Strength) -1.0) Hit%20Result))

(fn ConstructionScript
  (|CallParentFunction))