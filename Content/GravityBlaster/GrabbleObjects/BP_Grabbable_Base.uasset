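; BP_Grabbable_Base is the base Blueprint for objects that the gravity blaster pushes, pulls and releases through interface events.
; A push arms the object and enables CCD on its static mesh, while a pull disarms it and release is an empty stub.
; While armed, collisions fire the hit event, which disarms it a tick later and turns CCD off after a short delay.
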(event EventBeginPlay)

(event Collision|EventActorBeginOverlap
  (params (OtherActor :type Actor%20Object%20Reference)))

(event EventTick
  (params (DeltaSeconds :type Float%20%28single-precision%29)))

(event EventOnPushObjectBPI
  (Variables|Default|SetIsActive true)
  (bind _staticmesh (Variables|Default|GetStaticMesh)
    (:then
      (Class|PrimitiveComponent|SetUseCCD _staticmesh true "None"))
    (:else)))

(event EventOnPullObjectBPI
  (Variables|Default|SetIsActive false))

(event EventOnReleaseObjectBPI)

(event Collision|EventHit
  (params (MyComp :type Primitive%20Component%20Object%20Reference) (Other :type Actor%20Object%20Reference) (OtherComp :type Primitive%20Component%20Object%20Reference) (bSelfMoved :type Boolean) (HitLocation :type Vector :default "0, 0, 0") (HitNormal :type Vector :default "0, 0, 0") (NormalImpulse :type Vector :default "0, 0, 0") (Hit :type Hit%20Result%20Structure%20%28by%20ref%29))
  (if (Variables|Default|GetIsActive)
    (CallFunction|OnHitObjectBPI Hit)))

(event EventOnHitObjectBPI
  (params (Hit%20Result :type Hit%20Result%20Structure))
  (Utilities|FlowControl|DelayUntilNextTick)
  (Variables|Default|SetIsActive false)
  (Utilities|FlowControl|Delay 0.2)
  (bind _staticmesh (Variables|Default|GetStaticMesh)
    (:then
      (Class|PrimitiveComponent|SetUseCCD _staticmesh false "None"))
    (:else)))

(fn ConstructionScript)