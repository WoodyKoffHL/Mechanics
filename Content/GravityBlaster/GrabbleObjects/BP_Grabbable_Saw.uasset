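; BP_Grabbable_Saw is a grabbable saw object for the Gravity Blaster that deals slicing damage on contact.
; When pushed, it runs the parent push logic, then spins its static mesh with a mass-independent angular impulse around the mesh's up axis.
; Any actor that begins overlapping the mesh takes heavy point damage of the slice damage type, with the saw as damage causer.
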(event OnComponentBeginOverlap(StaticMesh)
  (params (OverlappedComponent :type Primitive%20Component%20Object%20Reference) (OtherActor :type Actor%20Object%20Reference) (OtherComp :type Primitive%20Component%20Object%20Reference) (OtherBodyIndex :type Integer) (bFromSweep :type Boolean) (SweepResult :type Hit%20Result%20Structure%20%28by%20ref%29))
  (Game|Damage|ApplyPointDamage OtherActor 2e+02 (Transformation|GetActorLocation) (Collision|MakeHitResult false false 0.0 0.0 "0, 0, 0" "0, 0, 0" "0,0,1" "0,0,1" 0 0) 0 self "/Game/GravityBlaster/Damage/DT_SliceDamage.DT_SliceDamage_C"))

(event EventBeginPlay
  (|CallParentFunction) ; This node is disabled and will not be called.\nDrag off pins to build functionality.
)

(event Collision|EventActorBeginOverlap
  (params (OtherActor :type Actor%20Object%20Reference))
  (|CallParentFunction OtherActor) ; This node is disabled and will not be called.\nDrag off pins to build functionality.
)

(event EventTick
  (params (DeltaSeconds :type Float%20%28single-precision%29))
  (|CallParentFunction DeltaSeconds) ; This node is disabled and will not be called.\nDrag off pins to build functionality.
)

(event EventOnPushObjectBPI
  (|CallParentFunction)
  (Class|PrimitiveComponent|AddAngularImpulseinDegrees (Variables|Default|GetStaticMesh) (* (Math|Vector|GetUpVector (Variables|Default|GetStaticMesh)) 3.6e+03) "None" true))

(fn ConstructionScript
  (|CallParentFunction))